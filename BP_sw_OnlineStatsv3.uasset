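; Server-side online stats reporter for Zomboy matches, sending player join/leave and kill feed events to a web API.
; On BeginPlay it fetches a game ID, using DownloadPak as the HTTP request for every call.
; Tick polls PlayerArray for joins and rebinds destroy and damage delegates; lethal point or listed damage types become kills (radial handler is never bound).
; Leaves are sent on player destruction, match end and actor destruction.
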(event `self.ReceiveBeginPlay`
  ;[1 1 1] Game Begin Play
  (`/Engine/EditorBlueprintResources/ActorMacros.Switch Has Authority`
    (:`Authority`
      (`|ExecutionSequence`
        (:`then_0`
          (bind _output_get (set `self.GameStartTime` (`GameplayStatics.GetRealTimeSeconds`))))
        (:`then_1`
          (bind _aszomboy_game_mode (cast `ZomboyGameMode` (`GameplayStatics.GetGameMode`)))
          (bind _returnvalue (`KismetTextLibrary.Conv_TextToString` (`ZomboyGameMode.GameModeDescription` _aszomboy_game_mode)))
          (set `self.GameMode` (`KismetStringLibrary.Replace` (`KismetStringLibrary.GetSubstring` _returnvalue 0 (`KismetStringLibrary.FindSubstring` _returnvalue " \n")) " " "%20")))
        (:`then_2`
          (bind (_httpresponsecode _contentlength _savepath) (`AsyncPakDownloader.DownloadPak` (`KismetStringLibrary.Concat_StrStr` (`self.CStatsAPIURL`) "getNewGameID") "gameID")
            (:`OnSuccess`
              (bind _outstringarray (`ZomboyBlueprintLibrary.LoadStringArrayFromFile` _savepath))
              (set `self.GameId` (`|GetArrayItem` _outstringarray)))))
        (:`then_3`
          (bind _aszomboy_game_state (cast `ZomboyGameState` (`GameplayStatics.GetGameState`)))
          (add `ZomboyGameState.ZomboymatchStateChangedDelegate` _aszomboy_game_state (delegate `ZBGameStateChanged`)))))))

(event `ZBGameStateChanged`
  (params (NewMatchState :type "EZomboyMatchState Enum" :default "BP_EMatchStateEnteringMap"))
  ;[1 1 1] Event when game ends to send leave
  (switch `EZomboyMatchState` NewMatchState
    (:`BP_EWaitingPostMatch`
      (for _array_element (`GameStateBase.PlayerArray` (`GameplayStatics.GetGameState`))
        (bind _aszomboy_player_state (cast `ZomboyPlayerState` _array_element))
        (`self.PlayerAddRemoveSend` (`PlayerState.GetPlayerName` _aszomboy_player_state) (`ZomboyBlueprintLibrary.GetCurrentMapName` _aszomboy_player_state) "false" (`KismetStringLibrary.Conv_IntToString` (`KismetMathLibrary.Conv_Int64ToInt` (`KismetMathLibrary.FTrunc64` (`PlayerState.Score` _aszomboy_player_state)))) (`self.GameMode`) (`self.CurrGameTime`) (`self.GameId`))))))

(event `self.ReceiveTick`
  (params (DeltaSeconds :type "Float (single-precision)"))
  ;[1 1 1] Tick
  (`|ExecutionSequence`
    (:`then_0`
      (bind _currgametime (`self.GetCurrGameTime`))
      (set `self.CurrGameTime` _currgametime))
    (:`then_1`
      (`TextRenderComponent.K2_SetText` (`self.DebugText`) (`KismetTextLibrary.Conv_StringToText` (`self.DebugTextValue`))))
    (:`then_2`
      (`self.CheckPlayers`))))

(event `AppendDebugLog`
  (params (NewText :type String))
  ;[1 1 1] Append Debug Log
  (set `self.DebugTextValue` (`KismetStringLibrary.Concat_StrStr` (`self.DebugTextValue`) " \n" NewText)))

(event `CheckPlayers`
  (bind _lastplayerids (`self.LastPlayerIds`))
  (bind _lastplayerids_2 (`self.LastPlayerIds`))
  ;[1 1 1] Check all Player Related Events
  (`/Engine/EditorBlueprintResources/ActorMacros.Switch Has Authority`
    (:`Authority`
      (`|ExecutionSequence`
        (:`then_0`
          ;[1 1 1] Player Add
          (for _array_element (`GameStateBase.PlayerArray` (`GameplayStatics.GetGameState`))
            (bind _playerid (`PlayerState.PlayerId` _array_element))
            (if (and (not (`PlayerState.bIsABot` _array_element)) (not (`KismetArrayLibrary.Array_Contains` _lastplayerids _playerid)))
              (`KismetArrayLibrary.Array_AddUnique` _lastplayerids _playerid)
              (bind _aszomboy_player_state (cast `ZomboyPlayerState` _array_element))
              (`self.PlayerAddRemoveSend` (`PlayerState.GetPlayerName` _aszomboy_player_state) (`ZomboyBlueprintLibrary.GetCurrentMapName` _aszomboy_player_state) "true" "0" (`self.GameMode`) (`self.CurrGameTime`) (`self.GameId`)))))
        (:`then_1`
          ;[1 1 1] Get Current Players
          (`|ExecutionSequence`
            (:`then_0`
              (`KismetArrayLibrary.Array_Clear` (`self.CurrentPlayerIds`)))
            (:`then_1`
              (for _array_element_2 (`GameStateBase.PlayerArray` (`GameplayStatics.GetGameState`))
                (`KismetArrayLibrary.Array_AddUnique` (`self.CurrentPlayerIds`) (`PlayerState.PlayerId` _array_element_2))))
            (:`then_2`
              ;[1 1 1] Player Remove
              (for _array_element_3 _lastplayerids_2
                (if (not (`KismetArrayLibrary.Array_Contains` (`self.CurrentPlayerIds`) _array_element_3))
                  (`KismetArrayLibrary.Array_RemoveItem` _lastplayerids_2 _array_element_3))))
            (:`then_3`
              (for _array_element_4 (`GameStateBase.PlayerArray` (`GameplayStatics.GetGameState`))
                (add `self.OnDestroyed` _array_element_4 (delegate `OnDestroyEventSend`))))))
        (:`then_2`
          ;[1 1 1] Bind KillFeed events
          (for _array_element_5 (`GameStateBase.PlayerArray` (`GameplayStatics.GetGameState`))
            (bind _aszomboy_vrcharacter (cast `ZomboyVRCharacter` (`Controller.K2_GetPawn` (`ZomboyBlueprintLibrary.GetOwningController` _array_element_5))))
            (add `self.OnTakePointDamage` _aszomboy_vrcharacter (delegate `OnPointDamageSend`))
            (add `self.OnTakeAnyDamage` _aszomboy_vrcharacter (delegate `OnAnyDamageSend`))))))))

(event `PlayerAddRemoveSend`
  (params (PlayerName :type String) (MapName :type String) (Added :type String) (Score :type String) (GameMode :type String) (GameTime :type String) (GameId :type String))
  ;[1 1 1] Send Player Add Remove
  (if (`KismetStringLibrary.NotEqual_StrStr` GameId)
    (`AsyncPakDownloader.DownloadPak` (`KismetStringLibrary.Concat_StrStr` (`self.CStatsURL`) "joinleave" "?" "pn=" PlayerName "&mn=" MapName "&added=" Added "&score=" Score "&gm=" GameMode "&gt=" GameTime "&gid=" GameId) "joinleave")))

(event `OnDestroyEventSend` :!signature `self.OnDestroyed`
  (params (DestroyedActor :type "Actor Object Reference"))
  ;[1 1 1] Player Remove
  (bind _aszomboy_game_state (cast `ZomboyGameState` (`GameplayStatics.GetGameState`)))
  (switch `EZomboyMatchState` (`ZomboyGameState.ZomboymatchState` _aszomboy_game_state)
    (:`BP_EMatchStateEnteringMap`
      _)
    (:`BP_EWaitingToStart`
      _)
    (:`BP_EInProgress`
      _)
    (:`BP_ELeavingMap`
      _)
    (:`BP_EAborted`
      _))
  (bind _aszomboy_player_state (cast `ZomboyPlayerState` (`Controller.PlayerState` (`ZomboyBlueprintLibrary.GetOwningController` DestroyedActor))))
  (`self.PlayerAddRemoveSend` (`PlayerState.GetPlayerName` _aszomboy_player_state) (`ZomboyBlueprintLibrary.GetCurrentMapName` _aszomboy_player_state) "false" (`KismetStringLibrary.Conv_IntToString` (`KismetMathLibrary.Conv_Int64ToInt` (`KismetMathLibrary.FTrunc64` (`PlayerState.Score` _aszomboy_player_state)))) (`self.GameMode`) (`self.CurrGameTime`) (`self.GameId`)))

(event `self.ReceiveDestroyed`
  ;[1 1 1] On BP Destroy Send all remaining Player Leave
  (`/Engine/EditorBlueprintResources/ActorMacros.Switch Has Authority`
    (:`Authority`
      (for _array_element (`GameStateBase.PlayerArray` (`GameplayStatics.GetGameState`))
        (bind _aszomboy_player_state (cast `ZomboyPlayerState` _array_element))
        (`self.PlayerAddRemoveSend` (`PlayerState.GetPlayerName` _aszomboy_player_state) (`ZomboyBlueprintLibrary.GetCurrentMapName` _aszomboy_player_state) "false" (`KismetStringLibrary.Conv_IntToString` (`KismetMathLibrary.Conv_Int64ToInt` (`KismetMathLibrary.FTrunc64` (`PlayerState.Score` _aszomboy_player_state)))) (`self.GameMode`) (`self.CurrGameTime`) (`self.GameId`))))))

(event `KillFeedSend`
  (params (KillerPlayerName :type String) (VictimPlayerName :type String) (IsHeadShot :type String) (MapName :type String) (BoneName :type String) (Damage :type String) (DamageType :type String) (Distance :type String) (GameId :type String) (GameMode :type String) (GameTime :type String) (KillerHealth :type String))
  ;[1 1 1] Send KillFeed
  (bind _aszomboy_game_state (cast `ZomboyGameState` (`GameplayStatics.GetGameState`)))
  (bind _returnvalue (`KismetSystemLibrary.GetDisplayName` (`ZomboyGameState.GetLoadoutPlan` _aszomboy_game_state)))
  (`AsyncPakDownloader.DownloadPak` (`KismetStringLibrary.Concat_StrStr` (`KismetStringLibrary.Concat_StrStr` (`self.CStatsURL`) "kill" "?" "kpn=" KillerPlayerName "&vpn=" VictimPlayerName "&ihs=" IsHeadShot "&mn=" MapName "&bn=" BoneName "&dmg=" Damage "&dmgtype=" DamageType "&dst=" Distance "&gid=" GameId "&gm=" GameMode "&gt=" GameTime) "&kh=" KillerHealth "&lo=" (`KismetStringLibrary.GetSubstring` _returnvalue 0 (`KismetStringLibrary.FindSubstring` _returnvalue "_LoadoutPlan")) "&ver=3") "killfeed"))

(event `OnRadialDamageSend` :!signature `self.OnTakeRadialDamage`
  (params (DamagedActor :type "Actor Object Reference") (Damage :type "Float (double-precision)") (DamageType :type "DamageType Object Reference") (Origin :type "Vector Structure") (HitInfo :type "HitResult Structure") (InstigatedBy :type "Controller Object Reference") (DamageCauser :type "Actor Object Reference"))
  (bind _returnvalue (`KismetSystemLibrary.GetDisplayName` DamageCauser))
  ;[1 1 1] Radial Damage
  (bind _aszomboy_vrcharacter (cast `ZomboyVRCharacter` DamagedActor))
  (if (and (`ZomboyCharacter.K2_IsAlive` _aszomboy_vrcharacter) (<= (`ZomboyCharacter.Health` _aszomboy_vrcharacter) Damage))
    (bind _aszomboy_player_state (cast `ZomboyPlayerState` (`Pawn.PlayerState` _aszomboy_vrcharacter)))
    (bind _aszomboy_vrcharacter_2 (cast `ZomboyVRCharacter` (`Controller.K2_GetPawn` InstigatedBy)))
    (bind _aszomboy_player_state_2 (cast `ZomboyPlayerState` (`Pawn.PlayerState` _aszomboy_vrcharacter_2)))
    (`self.KillFeedSend` (`PlayerState.GetPlayerName` _aszomboy_player_state_2) (`PlayerState.GetPlayerName` _aszomboy_player_state) (`KismetStringLibrary.Conv_BoolToString` false) (`ZomboyBlueprintLibrary.GetCurrentMapName` _aszomboy_player_state) (`KismetStringLibrary.Conv_NameToString` HitInfo_HitBoneName) (`KismetStringLibrary.Conv_DoubleToString` Damage) (`KismetStringLibrary.GetSubstring` _returnvalue 0 (`KismetStringLibrary.FindSubstring` _returnvalue "_C_")) (`KismetStringLibrary.Conv_DoubleToString` (`KismetMathLibrary.Vector_Distance` (`SceneComponent.K2_GetComponentLocation` (`Actor.RootComponent` DamagedActor)) (`SceneComponent.K2_GetComponentLocation` (`Actor.RootComponent` DamageCauser)))) (`self.GameId`) (`self.GameMode`) (`self.CurrGameTime`) (`KismetStringLibrary.Conv_DoubleToString` (`ZomboyCharacter.Health` _aszomboy_vrcharacter_2)))))

(event `OnPointDamageSend` :!signature `self.OnTakePointDamage`
  (params (DamagedActor :type "Actor Object Reference") (Damage :type "Float (double-precision)") (InstigatedBy :type "Controller Object Reference") (HitLocation :type "Vector Structure") (FHitComponent :type "PrimitiveComponent Object Reference") (BoneName :type Name) (ShotFromDirection :type "Vector Structure") (DamageType :type "DamageType Object Reference") (DamageCauser :type "Actor Object Reference"))
  (bind _returnvalue (`KismetSystemLibrary.GetDisplayName` DamageCauser))
  ;[1 1 1] PointDamage
  (bind _aszomboy_vrcharacter (cast `ZomboyVRCharacter` DamagedActor))
  (if (and (`ZomboyBlueprintLibrary.IsAlive` _aszomboy_vrcharacter) (<= (`ZomboyCharacter.Health` _aszomboy_vrcharacter) Damage))
    (bind _aszomboy_player_state (cast `ZomboyPlayerState` (`Pawn.PlayerState` _aszomboy_vrcharacter)))
    (bind _aszomboy_vrcharacter_2 (cast `ZomboyVRCharacter` (`Controller.K2_GetPawn` InstigatedBy)))
    (bind _aszomboy_player_state_2 (cast `ZomboyPlayerState` (`Pawn.PlayerState` _aszomboy_vrcharacter_2)))
    (`self.KillFeedSend` (`PlayerState.GetPlayerName` _aszomboy_player_state_2) (`PlayerState.GetPlayerName` _aszomboy_player_state) (`KismetStringLibrary.Conv_BoolToString` (`KismetTextLibrary.EqualEqual_TextText` (`KismetTextLibrary.Conv_NameToText` BoneName) "Head")) (`ZomboyBlueprintLibrary.GetCurrentMapName` _aszomboy_player_state) (`KismetStringLibrary.Conv_NameToString` BoneName) (`KismetStringLibrary.Conv_DoubleToString` Damage) (`KismetStringLibrary.GetSubstring` _returnvalue 0 (`KismetStringLibrary.FindSubstring` _returnvalue "_C_")) (`KismetStringLibrary.Conv_DoubleToString` (`KismetMathLibrary.Vector_Distance` (`SceneComponent.K2_GetComponentLocation` (`Actor.RootComponent` DamagedActor)) (`SceneComponent.K2_GetComponentLocation` (`Actor.RootComponent` DamageCauser)))) (`self.GameId`) (`self.GameMode`) (`self.CurrGameTime`) (`KismetStringLibrary.Conv_DoubleToString` (`ZomboyCharacter.Health` _aszomboy_vrcharacter_2)))))

(event `OnAnyDamageSend` :!signature `self.OnTakeAnyDamage`
  (params (DamagedActor :type "Actor Object Reference") (Damage :type "Float (double-precision)") (DamageType :type "DamageType Object Reference") (InstigatedBy :type "Controller Object Reference") (DamageCauser :type "Actor Object Reference"))
  (bind _returnvalue (`KismetSystemLibrary.GetDisplayName` DamageCauser))
  ;[1 1 1] Other Damage
  (if (`KismetArrayLibrary.Array_Contains` (`self.OtherDamageTypes`) (`KismetSystemLibrary.GetClassDisplayName` (`GameplayStatics.GetObjectClass` DamageType)))
    (bind _aszomboy_vrcharacter (cast `ZomboyVRCharacter` DamagedActor))
    (if (and (`ZomboyCharacter.K2_IsAlive` _aszomboy_vrcharacter) (<= (`ZomboyCharacter.Health` _aszomboy_vrcharacter) Damage))
      (bind _aszomboy_player_state (cast `ZomboyPlayerState` (`Pawn.PlayerState` _aszomboy_vrcharacter)))
      (bind _aszomboy_vrcharacter_2 (cast `ZomboyVRCharacter` (`Controller.K2_GetPawn` InstigatedBy)))
      (bind _aszomboy_player_state_2 (cast `ZomboyPlayerState` (`Pawn.PlayerState` _aszomboy_vrcharacter_2)))
      (`self.KillFeedSend` (`PlayerState.GetPlayerName` _aszomboy_player_state_2) (`PlayerState.GetPlayerName` _aszomboy_player_state) (`KismetStringLibrary.Conv_BoolToString` false) (`ZomboyBlueprintLibrary.GetCurrentMapName` _aszomboy_player_state) "none" (`KismetStringLibrary.Conv_DoubleToString` Damage) (`KismetStringLibrary.GetSubstring` _returnvalue 0 (`KismetStringLibrary.FindSubstring` _returnvalue "_C_")) (`KismetStringLibrary.Conv_DoubleToString` (`KismetMathLibrary.Vector_Distance` (`SceneComponent.K2_GetComponentLocation` (`Actor.RootComponent` DamagedActor)) (`SceneComponent.K2_GetComponentLocation` (`Actor.RootComponent` DamageCauser)))) (`self.GameId`) (`self.GameMode`) (`self.CurrGameTime`) (`KismetStringLibrary.Conv_DoubleToString` (`ZomboyCharacter.Health` _aszomboy_vrcharacter_2))))))

(fn `GetCurrGameTime`
  (returns (CurrGameTime :type String))
  (return (`KismetStringLibrary.Conv_DoubleToString` (/ (`KismetMathLibrary.Conv_IntToDouble` (`KismetMathLibrary.Round` (* (- (`GameplayStatics.GetRealTimeSeconds`) (`self.GameStartTime`)) 10.0))) 10.0))))

(fn `ServerSetPlayerBodyData`
  (params (PlayerBodyData :type "ZomboyPlayerBodyData Object Reference")))

(fn `UserConstructionScript`)